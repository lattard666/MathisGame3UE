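; Game flow manager that runs the level loop: loading, gameplay, game over and level complete.
; On BeginPlay it caches the player and controller, creates the flow UI and streams the first level as a level instance.
; A state setter drives UI and input mode, while Tick accumulates playtime during gameplay.
; Setting a start position respawns the player, and the next step reloads, advances or quits after the last level.
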(event EventBeginPlay
  (GameFlow|InitGameManager))

(event EventTick
  (params (DeltaSeconds :type Float%20%28single-precision%29))
  (if (Utilities|Enum|Equal(Enum) (Variables|GameFlowManager|CachedVariables|GetStateCurrent) "NewEnumerator1")
    (Variables|GameFlowManager|CachedVariables|SetPlaytime (+ DeltaSeconds (Variables|GameFlowManager|CachedVariables|GetPlaytime)))))

(fn ConstructionScript
  (Variables|GameFlowManager|CachedVariables|SetStateCurrent "NewEnumerator0"))

(fn LoadLevel
  (params (LevelIndex :type Integer))
  (Utilities|FlowControl|Sequence
    (:then_0
      (Variables|GameFlowManager|CachedVariables|SetPlaytime 0.0))
    (:then_1
      (Utils|SetState "NewEnumerator4"))
    (:then_2
      (bind _returnvalue (Class|LevelStreamingDynamic|LoadLevelInstancebySoftObjectPtr (Utilities|Array|Get(acopy) (Variables|GameFlowManager|CachedVariables|GetLevels) LevelIndex) "0, 0, 0" "0, 0, 0" "" 0))
      (Variables|GameFlowManager|CachedVariables|SetCurrentLevel _returnvalue))))

(fn ReloadLevel
  (Utilities|FlowControl|Sequence
    (:then_0
      (Levels|UnloadCurrentLevel))
    (:then_1
      (Levels|LoadLevel (Variables|GameFlowManager|CachedVariables|GetCurrentLevelIndex)))))

(fn UnloadCurrentLevel
  (Class|LevelStreaming|SetIsRequestingUnloadandRemoval (Variables|GameFlowManager|CachedVariables|GetCurrentLevel) true))

(fn OnGameplay
  (Utilities|FlowControl|Sequence
    (:then_0
      (Default|OnGameplay (Variables|Default|GetGame%20Flow%20UIRef)))
    (:then_1
      (Utils|ShowMouseCursor false))))

(fn OnGameOver
  (Utilities|FlowControl|Sequence
    (:then_0
      (Default|OnGameplayEnd (Variables|Default|GetGame%20Flow%20UIRef) true (Variables|GameFlowManager|CachedVariables|GetPlaytime)))
    (:then_1
      (Utils|ShowMouseCursor true))))

(fn OnLevelComplete
  (Utilities|FlowControl|Sequence
    (:then_0
      (Default|OnGameplayEnd (Variables|Default|GetGame%20Flow%20UIRef) false (Variables|GameFlowManager|CachedVariables|GetPlaytime)))
    (:then_1
      (Utils|ShowMouseCursor false))
    (:then_2
      (Levels|UnloadCurrentLevel))))

(fn OnLoadingLevel
  (Default|OnLoadingLevel (Variables|Default|GetGame%20Flow%20UIRef)))

(fn InitGameManager
  (Utilities|FlowControl|Sequence
    (:then_0
      (Variables|GameFlowManager|CachedVariables|GetPlayerRef
        (:then)
        (:else
          (bind _outactors (Actor|GetAllActorsOfClass "/Game/Player/BP_Player.BP_Player_C"))
          (bind _output_get (Variables|GameFlowManager|CachedVariables|SetPlayerRef (Utilities|Array|Get(acopy) _outactors)))
          (bind _asbp_player_controller (Utilities|Casting|CastToBP_PlayerController (Pawn|GetController _output_get)))
          (Variables|GameFlowManager|CachedVariables|SetPlayerControllerRef _asbp_player_controller))))
    (:then_1
      (Variables|GameFlowManager|CachedVariables|GetGameFlowUIRef
        (:then)
        (:else
          (bind _returnvalue (UserInterface|CreateWidget "/Game/_Core/_Widgets/WBP_GameFlowUI.WBP_GameFlowUI_C" (Variables|GameFlowManager|CachedVariables|GetPlayerControllerRef)))
          (Variables|Default|SetGame%20Flow%20UIRef _returnvalue)
          (Utilities|FlowControl|Sequence
            (:then_0
              (Default|InitWidget (Variables|Default|GetGame%20Flow%20UIRef) self (Variables|GameFlowManager|CachedVariables|GetPlayerRef)))
            (:then_1
              (UserInterface|Viewport|AddtoViewport (Variables|Default|GetGame%20Flow%20UIRef) 0))))))
    (:then_2
      (Variables|GameFlowManager|CachedVariables|SetPlaytime 0.0))
    (:then_3
      (Variables|GameFlowManager|CachedVariables|SetCurrentLevelIndex 0))
    (:then_4
      (Levels|LoadLevel (Variables|GameFlowManager|CachedVariables|GetCurrentLevelIndex)))))

(fn PerformNextStep
  (if (Utilities|Enum|Equal(Enum) (Variables|GameFlowManager|CachedVariables|GetStateCurrent) "NewEnumerator2")
    (Levels|ReloadLevel)
    (elif (Utils|IsLastLevel)
      (Game|QuitGame 0 "Quit" false)
      (else
        (bind _result (Math|Integer|IncrementInt (Variables|GameFlowManager|CachedVariables|GetCurrentLevelIndex))
          (:%20%20
            (Levels|LoadLevel _result)))))))

(fn SetStartPosition
  (params (StartPosition :type BP%20Start%20Position%20Object%20Reference))
  (Variables|GameFlowManager|CachedVariables|SetCurrentStartPos StartPosition)
  (Utilities|FlowControl|Sequence
    (:then_0
      (Utils|RespawnPlayer))
    (:then_1
      (Utils|SetState "NewEnumerator1"))))

(fn SetState
  (params (NewState :type EGameState%20Enum :default "NewEnumerator0"))
  (bind _output_get (Variables|GameFlowManager|CachedVariables|SetStateCurrent NewState))
  (switch Utilities|FlowControl|Switch|SwitchonEGameState _output_get
    (:NewEnumerator1
      (CallBacks|OnGameplay))
    (:NewEnumerator2
      (CallBacks|OnGameOver))
    (:NewEnumerator3
      (CallBacks|OnLevelComplete))
    (:NewEnumerator4
      (CallBacks|OnLoadingLevel))))

(fn IsLastLevel
  (return (== (- (Utilities|Array|Length (Variables|GameFlowManager|CachedVariables|GetLevels)) 1) (Variables|GameFlowManager|CachedVariables|GetCurrentLevelIndex))))

(fn RespawnPlayer
  (bind _playerref (Variables|GameFlowManager|CachedVariables|GetPlayerRef))
  (Utilities|FlowControl|Sequence
    (:then_0
      (Default|InitPlayer _playerref))
    (:then_1
      (Default|ForceTransform _playerref (Transformation|GetActorTransform (Variables|GameFlowManager|CachedVariables|GetCurrentStartPos))))))

(fn ShowMouseCursor
  (params (bShow :type Boolean))
  (bind _playercontrollerref (Variables|GameFlowManager|CachedVariables|GetPlayerControllerRef))
  (bind _playercontrollerref_2 (Variables|GameFlowManager|CachedVariables|GetPlayerControllerRef))
  (if bShow
    (Input|SetInputModeUIOnly _playercontrollerref_2 (Variables|GameFlowManager|CachedVariables|GetGameFlowUIRef) "LockAlways")
    (Variables|/Script/Engine.PlayerController|SetbShowMouseCursor _playercontrollerref_2 true)
    (else
      (Input|SetInputModeGameOnly _playercontrollerref)
      (Variables|/Script/Engine.PlayerController|SetbShowMouseCursor _playercontrollerref false))))

(fn OnLevelLoaded
  (Utils|SetState "NewEnumerator1"))

(fn OnLevelEnd
  (params (Is%20Complete :type Boolean))
  (if Is%20Complete
    (Utils|SetState "NewEnumerator3")
    (else
      (Utils|SetState "NewEnumerator2"))))