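; BP_ExplosiveBarrel is a throwable gravity-target barrel that explodes when its health runs out or when a throw ends.
; Incoming damage lowers Health, and both that path and OnThrowEnd, after its parent call, lead into Explode.
; Explode uses IsAlive to fire only once, spawns BP_Explosion at the visual's location with the barrel's damage and radius, then destroys the actor.
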(event EventTakeDamage
  (params (Damage :type Float%20%28single-precision%29))
  (CallFunction|TakeDamageInternal Damage))

(fn ConstructionScript
  (|CallParentFunction))

(fn TakeDamageInternal
  (params (Damage :type Float%20%28single-precision%29))
  (bind _output_get (Variables|ExplosiveBarrel|SetHealth (- (Variables|ExplosiveBarrel|GetHealth) Damage)))
  (if (and (<= _output_get 0.0) (Variables|ExplosiveBarrel|CachedVariables|GetbIsAlive))
    (CallFunction|Explode)))

(fn Explode
  (if (Variables|ExplosiveBarrel|CachedVariables|GetbIsAlive)
    (Variables|ExplosiveBarrel|CachedVariables|SetbIsAlive false)
    (Game|SpawnActorfromClass "/Game/LDis/GravityTargets/BP_Explosion.BP_Explosion_C" (Math|Transform|MakeTransform (Transformation|GetWorldLocation (Variables|Default|GetVisual)) "0, 0, 0" "1,1,1") "AlwaysSpawn" 0 (Variables|ExplosiveBarrel|GetExplosionDamage) (Variables|ExplosiveBarrel|GetExplosionRadius) 0)
    (Actor|DestroyActor)))

(fn OnThrowEnd
  (params (Hit :type Hit%20Result%20Structure))
  (|CallParentFunction Hit)
  (CallFunction|Explode))