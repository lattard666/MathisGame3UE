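; Base actor for objects that can be grabbed, dropped and thrown as gravity targets.
; BeginPlay stores the visual's scale, applies a mass override and sets Idle; SetState then routes grab travel, grabbed and thrown states to hook functions.
; Tick updates grab travel, and a hit while Idle calls OnThrowEnd.
; Grab, drop and throw events only print debug text, while travel, physics, reset and state hooks are empty stubs.
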(event OnComponentHit(Visual)
  (params (HitComponent :type Primitive%20Component%20Object%20Reference) (OtherActor :type Actor%20Object%20Reference) (OtherComp :type Primitive%20Component%20Object%20Reference) (NormalImpulse :type Vector :default "0, 0, 0") (Hit :type Hit%20Result%20Structure%20%28by%20ref%29))
  (if (Utilities|Enum|Equal(Enum) (Variables|GravityTarget|CachedVariable|GetCurrentState) "NewEnumerator0")
    (Calibacks|OnThrowEnd)))

(event EventBeginPlay
  (Utils|InitTarget))

(event EventTick
  (params (DeltaSeconds :type Float%20%28single-precision%29))
  (switch Utilities|FlowControl|Switch|SwitchonEGravityTargetsState (Variables|GravityTarget|CachedVariable|GetCurrentState)
    (:NewEnumerator1
      (GamePlay|UpdateGrabTravel DeltaSeconds))))

(fn ConstructionScript)

(fn OnGrabbed
  (params (GrabLocaltion :type Scene%20Component%20Object%20Reference))
  (Utilities|FlowControl|Sequence
    (:then_0
      (Development|PrintString (Utilities|String|Append "Gravity Target" (Utilities|GetDisplayName self) "-GRABBED")))))

(fn OnDropped
  (Utilities|FlowControl|Sequence
    (:then_0
      (Development|PrintString (Utilities|String|Append "Gravity Target" (Utilities|GetDisplayName self) "-DROPPED") true true "(R=1.000000,G=0.000000,B=0.454612,A=1.000000)"))))

(fn OnThrown
  (params (ThrowVector :type Vector))
  (Utilities|FlowControl|Sequence
    (:then_0
      (Development|PrintString (Utilities|String|Append "Gravity Target" (Utilities|GetDisplayName self) "-THROW") true true "(R=0.000000,G=1.000000,B=0.046065,A=1.000000)"))))

(fn UpdateGrabTravel
  (params (DeltaTime :type Float%20%28single-precision%29)))

(fn InitTarget
  (bind _visual (Variables|Default|GetVisual))
  (Utilities|FlowControl|Sequence
    (:then_0
      (Variables|GravityTarget|CachedVariable|SetGrabFinalLocation 0))
    (:then_1
      (Variables|GravityTarget|CachedVariable|SetGrabTravelPercent 0.0))
    (:then_2
      (Variables|GravityTarget|CachedVariable|SetScaleDefault (Transformation|GetWorldScale _visual)))
    (:then_3
      (Class|PrimitiveComponent|SetMassOverrideinKg _visual "None" (Variables|GravityTarget|GetTargetMass) true))
    (:then_4
      (Utils|SetState "NewEnumerator0"))))

(fn SetState
  (params (NewState :type EGravityTargetsState%20Enum :default "NewEnumerator0"))
  (bind _output_get (Variables|GravityTarget|CachedVariable|SetCurrentState NewState))
  (switch Utilities|FlowControl|Switch|SwitchonEGravityTargetsState _output_get
    (:NewEnumerator1
      (Calibacks|OnGrabTravelStart))
    (:NewEnumerator2
      (Calibacks|OnGrabTravelEnd))
    (:NewEnumerator3
      (Calibacks|OnThrowStart))))

(fn ActivatePhysics
  (params (bActivate :type Boolean)))

(fn ResetActor)

(fn OnGrabTravelStart)

(fn OnGrabTravelEnd)

(fn OnThrowStart)

(fn OnThrowEnd)