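; BP_Explosion is an explosion actor that deals area damage for a limited lifespan.
; On BeginPlay it scales its root uniformly by Radius, clears the damaged-actor list, then destroys itself once Lifespan elapses.
; Actors that begin overlapping VisualCollision receive a TakeDamageMessage with Damage, and the DamagedActors list ensures each is hit only once.
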(event OnComponentBeginOverlap(VisualCollision)
  (params (OverlappedComponent :type Primitive%20Component%20Object%20Reference) (OtherActor :type Actor%20Object%20Reference) (OtherComp :type Primitive%20Component%20Object%20Reference) (OtherBodyIndex :type Integer) (bFromSweep :type Boolean) (SweepResult :type Hit%20Result%20Structure%20%28by%20ref%29))
  (if (not (Utilities|Set|Contains (Variables|Explosion|CachedVariables|GetDamagedActors) OtherActor))
    (Utilities|FlowControl|Sequence
      (:then_0
        (Utilities|Set|Add (Variables|Explosion|CachedVariables|GetDamagedActors) OtherActor))
      (:then_1
        (Class|IDestructible|TakeDamage(Message) OtherActor (Variables|Explosion|GetDamage))))))

(event EventBeginPlay
  (CallFunction|InitExplosion)
  (Utilities|FlowControl|Delay (Variables|Explosion|GetLifespan))
  (Actor|DestroyActor))

(fn ConstructionScript)

(fn InitExplosion
  (bind _radius (Variables|Explosion|GetRadius))
  (Utilities|FlowControl|Sequence
    (:then_0
      (Transformation|SetWorldScale3D (Variables|Default|GetDefaultSceneRoot) (Math|Vector|MakeVector _radius _radius _radius)))
    (:then_1
      (Utilities|Set|Clear (Variables|Explosion|CachedVariables|GetDamagedActors)))))