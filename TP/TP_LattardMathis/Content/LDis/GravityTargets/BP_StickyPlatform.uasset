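; BP_StickyPlatform is a throwable gravity target that sticks to the surface it hits, judging by its name and folder.
; It overrides OnThrowEnd: after the parent logic, it disables physics and teleports the root to the hit location, aligning its X axis with the surface normal.
; It then sets the visual's collision profile to the default one; the event graph is otherwise unused.
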(event EventBeginPlay
  (|CallParentFunction) ; This node is disabled and will not be called.\nDrag off pins to build functionality.
)

(event Collision|EventActorBeginOverlap
  (params (OtherActor :type Actor%20Object%20Reference)))

(event EventTick
  (params (DeltaSeconds :type Float%20%28single-precision%29))
  (|CallParentFunction DeltaSeconds) ; This node is disabled and will not be called.\nDrag off pins to build functionality.
)

(fn ConstructionScript
  (|CallParentFunction))

(fn OnThrowEnd
  (params (Hit :type Hit%20Result%20Structure))
  (bind (_bblockinghit _binitialoverlap _time _distance _location _impactpoint _normal) (Collision|BreakHitResult Hit))
  (|CallParentFunction Hit)
  (Utilities|FlowControl|Sequence
    (:then_0
      (CallFunction|ActivatePhysics false))
    (:then_1
      (Transformation|SetWorldLocationAndRotation (Variables|Default|GetDefaultSceneRoot) _location (Math|Conversions|RotationFromXVector _normal) false true))
    (:then_2
      (Collision|SetCollisionProfileName (Variables|Default|GetVisual) (Variables|Default|GetCollisionProfileDefault) true :!class /Script/Engine.PrimitiveComponent))))