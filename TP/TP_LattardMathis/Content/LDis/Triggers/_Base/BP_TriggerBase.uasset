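; BP_TriggerBase is a base trigger actor that reacts to other actors entering and leaving its overlap.
; Its ActorBeginOverlap and ActorEndOverlap events forward the other actor to the OnActorTriggerEnter and OnActorTriggerLeave functions.
; Both functions only print red French debug messages with the actor's display name, and both label it "[Player][Enter]" without filtering for the player.
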(event Collision|EventActorBeginOverlap
  (params (OtherActor :type Actor%20Object%20Reference))
  (CallFunction|OnActorTriggerEnter OtherActor))

(event Collision|EventActorEndOverlap
  (params (OtherActor :type Actor%20Object%20Reference))
  (CallFunction|OnActorTriggerLeave OtherActor))

(fn ConstructionScript)

(fn OnActorTriggerEnter
  (params (Actor :type Actor%20Object%20Reference))
  (Development|PrintString (Utilities|String|Append "[Player][Enter] Je suis dedans" (Utilities|GetDisplayName Actor)) true true "(R=1.000000,G=0.007843,B=0.000000,A=1.000000)"))

(fn OnActorTriggerLeave
  (params (Actor :type Actor%20Object%20Reference))
  (Development|PrintString (Utilities|String|Append "[Player][Enter] Je suis plus dedans" (Utilities|GetDisplayName Actor)) true true "(R=1.000000,G=0.007843,B=0.000000,A=1.000000)"))