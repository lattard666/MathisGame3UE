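; BP_CollectibleBase is a collectible trigger actor that gives the player a key.
; Tick calls CollectKey whenever PlayerInTrigger is valid, through a branch hardcoded to true.
; CollectKey adds one key to that player, clears CanCollect and destroys the actor.
; RegisterManager stores an objective manager reference, which is not used elsewhere in this Blueprint.
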(event EventRegisterManager
  (params (Manager :type BP%20Objective%20Manager%20Object%20Reference))
  (Variables|Default|SetObjectiveManagerRef Manager))

(event EventTick
  (params (DeltaSeconds :type Float%20%28single-precision%29))
  (Variables|Default|GetPlayerInTrigger
    (:then
      (if true
        (CallFunction|CollectKey)))
    (:else)))

(fn ConstructionScript
  (|CallParentFunction))

(fn CollectKey
  (Default|AddKeys (Variables|Default|GetPlayerInTrigger) 1)
  (Variables|Default|SetbCanCollect false)
  (Actor|DestroyActor))