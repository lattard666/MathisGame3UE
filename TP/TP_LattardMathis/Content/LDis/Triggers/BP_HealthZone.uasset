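; BP_HealthZone is a trigger zone that either damages or heals the player inside it over time, chosen by the BisDamage flag.
; Each tick, while PlayerInTrigger is valid, ApplyZoneEffect calls TakeDamage or AddHealth with the per-second rate scaled by delta time.
; The construction script runs the parent's version, then sets the Visual's damage or heal material to match the flag.
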(event EventTick
  (params (DeltaSeconds :type Float%20%28single-precision%29))
  (Variables|Default|GetPlayerInTrigger
    (:then
      (CallFunction|ApplyZoneEffect DeltaSeconds))
    (:else)))

(fn ConstructionScript
  (|CallParentFunction)
  (if (Variables|Default|GetbisDamage)
    (LocalVariables|Setl_material (Variables|Default|GetMatDamage))
    (else
      (LocalVariables|Setl_material (Variables|Default|GetMatHeal))))
  (Rendering|Material|SetMaterial (Variables|Default|GetVisual) 0 (LocalVariables|Getl_material)))

(fn ApplyZoneEffect
  (params (DeltaTime :type Float%20%28single-precision%29))
  (bind _playerintrigger (Variables|Default|GetPlayerInTrigger))
  (LocalVariables|Setl_deltaTime DeltaTime)
  (if (Variables|Default|GetbisDamage)
    (Default|TakeDamage _playerintrigger (* (Variables|Default|GetDamagePerSecond) (LocalVariables|Getl_deltaTime)))
    (else
      (Default|AddHealth _playerintrigger (* (LocalVariables|Getl_deltaTime) (Variables|Default|GetHealPerSecond))))))