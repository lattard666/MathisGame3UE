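; Key-locked door actor that opens when the player in its trigger has a key, consuming it and revealing the Key component.
; Tick polls for the key and starts a one-time sequence: delay, opening timeline, then a delayed closing timeline.
; Timeline updates nudge the actor one unit along world Y per frame, reversed for closing.
; A registered objective manager receives target-complete on unlock and every opening update.
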(event EventBeginPlay
  (Utilities|FlowControl|Sequence
    (:then_0
      (Variables|Default|SetbMustOpen false))
    (:then_1
      (Variables|Default|SetbisOpen false))))

(event EventRegisterManager
  (params (Manager :type BP%20Objective%20Manager%20Object%20Reference))
  (Variables|Default|SetObjectiveManagerRef Manager))

(event EventTick
  (params (DeltaSeconds :type Float%20%28single-precision%29))
  (Variables|Default|SetDeltaTime DeltaSeconds)
  (if (Variables|Default|GetbMustOpen)
    (Variables|Default|SetbMustOpen false)
    (if (not (Variables|Default|GetbisOpen))
      (Variables|Default|SetbisOpen true)
      (Utilities|FlowControl|Delay (Variables|Default|GetDelayBeforeOpen))
      (Timeline|Timeline Play
        (:Update
          (CallFunction|OpenDoor)
          (Utilities|FlowControl|Delay (Variables|Default|GetDelayBeforeOpen))
          (Timeline|Timeline_0 Play
            (:Update
              (CallFunction|CloseDOor))))))
    (else
      (Variables|Default|GetPlayerInTrigger
        (:then
          (CallFunction|CheckOpenDoor))
        (:else)))))

(fn ConstructionScript
  (|CallParentFunction))

(fn CheckOpenDoor
  (bind _playerintrigger (Variables|Default|GetPlayerInTrigger))
  (if (Default|HasKey _playerintrigger)
    (Default|RemoveKeys _playerintrigger 1)
    (Variables|Default|SetbMustOpen true)
    (Rendering|SetVisibility (Variables|Default|Getkey) true false)
    (bind _objectivemanagerref (Variables|Default|GetObjectiveManagerRef)
      (:then
        (Default|OnTargetComplete _objectivemanagerref))
      (:else))))

(fn OpenDoor
  (bind _defaultsceneroot (Variables|Default|GetDefaultSceneRoot))
  (bind _returnvalue (Transformation|GetWorldTransform _defaultsceneroot))
  (Utilities|FlowControl|Sequence
    (:then_0
      (bind _objectivemanagerref (Variables|Default|GetObjectiveManagerRef)
        (:then
          (Default|OnTargetComplete _objectivemanagerref))
        (:else)))
    (:then_1
      (Transformation|SetActorTransform (Math|Transform|MakeTransform (+ "0,1.000000,0" (.location _returnvalue)) (.rotation _returnvalue) (.scale _returnvalue))))))

(fn CloseDOor
  (bind _defaultsceneroot (Variables|Default|GetDefaultSceneRoot))
  (bind _returnvalue (Transformation|GetWorldTransform _defaultsceneroot))
  (Transformation|SetActorTransform (Math|Transform|MakeTransform (+ (.location _returnvalue) "0,-1.000000,0") (.rotation _returnvalue) (.scale _returnvalue))))