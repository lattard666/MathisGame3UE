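; BP_Switch is a trigger switch that shows an on or off material and opens a door through its Action reference.
; OnInteraction sets the Interaction flag from its input, while Tick sets it every frame from whether PlayerInTrigger is valid.
; Both feed DoSwitchInternal, which swaps the Switch material and calls OpenDoor whenever the flag is true, so repeatedly while a player stays inside.
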(event EventTick
  (params (DeltaSeconds :type Float%20%28single-precision%29))
  (Variables|Default|GetPlayerInTrigger
    (:then
      (Variables|Default|SetInteraction true))
    (:else
      (Variables|Default|SetInteraction false)))
  (CallFunction|DoSwitchInternal))

(event EventOnInteraction
  (params (Intraction :type Boolean))
  (Variables|Default|SetInteraction Intraction)
  (CallFunction|DoSwitchInternal))

(fn ConstructionScript
  (|CallParentFunction))

(fn DoSwitchInternal
  (if (Variables|Default|GetInteraction)
    (LocalVariables|Setl_material (Variables|Default|GetOn))
    (else
      (LocalVariables|Setl_material (Variables|Default|Getoff))))
  (Rendering|Material|SetMaterial (Variables|Default|GetSwitch) 0 (LocalVariables|Getl_material))
  (if (Variables|Default|GetInteraction)
    (Default|OpenDoor (Variables|Default|GetAction))))