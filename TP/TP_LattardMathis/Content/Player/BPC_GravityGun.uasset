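; Player component that implements a gravity gun for grabbing, dropping and throwing BP_GravityTargetBase actors.
; Each tick it line traces from the player camera along its forward vector, caching any gravity target hit as the one in sight, with a per-frame debug draw.
; Grab toggles between holding the sighted target at the player's grab socket and dropping it; throw launches the held target along camera forward scaled by a throw force.
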(event EventBeginPlay)

(event EventTick
  (params (DeltaSeconds :type Float%20%28single-precision%29))
  (CallFunction|UpdateTarget))

(fn InitGravityGun
  (params (BP_Player :type BP%20Player%20Object%20Reference))
  (Utilities|FlowControl|Sequence
    (:then_0
      (Variables|GravityGun|cachedVariable|SetPlayerRef BP_Player))
    (:then_1
      (Variables|GravityGun|cachedVariable|SetGravityTargetCurrent 0))
    (:then_2
      (Variables|GravityGun|cachedVariable|SetGravityTargetInSight 0))))

(fn UpdateTarget
  (bind _playerref (Variables|GravityGun|cachedVariable|GetPlayerRef))
  (bind _camera (Variables|/Game/Player/BP_Player.BP_Player_C|GetCamera _playerref))
  (bind _returnvalue (Transformation|GetWorldLocation _camera))
  (bind _outhit (Collision|LineTraceByChannel _returnvalue (+ _returnvalue (* (Math|Vector|GetForwardVector _camera) (Variables|GravityGun|cachedVariable|GetLineTraceLength))) "TraceTypeQuery3" false 0 "ForOneFrame"))
  (if (.bBlockingHit (Collision|BreakHitResult _outhit))
    (bind _asbp_gravity_target_base (Utilities|Casting|CastToBP_GravityTargetBase (.HitActor (Collision|BreakHitResult _outhit)))
      (:then
        (Variables|GravityGun|cachedVariable|SetGravityTargetInSight _asbp_gravity_target_base))
      (:CastFailed
        (Variables|GravityGun|cachedVariable|SetGravityTargetInSight 0 :!label _label)))
    (else
      (goto _label))))

(fn OnGrabPressed
  (bind _gravitytargetcurrent (Variables|GravityGun|cachedVariable|GetGravityTargetCurrent)
    (:then
      (Default|OnDropped _gravitytargetcurrent)
      (Variables|GravityGun|cachedVariable|SetGravityTargetCurrent 0))
    (:else
      (bind _gravitytargetinsight (Variables|GravityGun|cachedVariable|GetGravityTargetInSight)
        (:then
          (bind _output_get (Variables|GravityGun|cachedVariable|SetGravityTargetCurrent _gravitytargetinsight))
          (Default|OnGrabbed _output_get (Default|GetGrabSocket (Variables|GravityGun|cachedVariable|GetPlayerRef))))
        (:else)))))

(fn OnThrowPressed
  (bind _gravitytargetcurrent (Variables|GravityGun|cachedVariable|GetGravityTargetCurrent)
    (:then
      (Default|OnThrown _gravitytargetcurrent (* (Math|Vector|GetForwardVector (Variables|/Game/Player/BP_Player.BP_Player_C|GetCamera (Variables|GravityGun|cachedVariable|GetPlayerRef))) (Variables|GravityGun|GetGravityThrowForce)))
      (Variables|GravityGun|cachedVariable|SetGravityTargetCurrent 0))
    (:else)))