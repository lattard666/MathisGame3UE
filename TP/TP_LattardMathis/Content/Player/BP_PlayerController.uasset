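; BP_PlayerController is the player controller that tracks jump input and initializes the controlled BP_Player pawn.
; On BeginPlay, InitController casts and caches the pawn as PlayerRef, then sets its starting state through SetState.
; Jump press and release only toggle the JumpPressed flag, with no jump logic in this controller.
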(event EventBeginPlay
  (CallFunction|InitController))

(event EventTick
  (params (DeltaSeconds :type Float%20%28single-precision%29)))

(event Input|ActionEvents|InputActionJump
  (params (Key :type Key%20Structure :default "None"))
  (:Pressed
    (Variables|Default|SetbJumpPressed true))
  (:Released
    (Variables|Default|SetbJumpPressed false)))

(fn ConstructionScript)

(fn InitController
  (Utilities|FlowControl|Sequence
    (:then_0
      (bind _asbp_player (Utilities|Casting|CastToBP_Player (Pawn|GetControlledPawn)))
      (Variables|Default|SetPlayerRef _asbp_player))
    (:then_1
      (Default|SetState (Variables|Default|GetPlayerRef) "NewEnumerator0"))))