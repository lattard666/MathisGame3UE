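; Player character Blueprint that provides movement, aiming, jump, stamina-limited dash, health, key inventory and a gravity gun.
; It exposes action functions for outside callers, with jump and dash using LaunchCharacter and grab/throw forwarded to the BPCGravityGun component.
; Tick regenerates dash stamina, while InitPlayer, jumping and lethal damage set a state enum that is printed for debugging.
; ForceTransform teleports the character, offsetting by the body's relative location and overriding control rotation.
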(event EventTakeDamage
  (params (Damage :type Float%20%28single-precision%29))
  (Health|TakeDamageInterface Damage))

(event EventTick
  (params (DeltaSeconds :type Float%20%28single-precision%29))
  (if (>= 1e+02 (+ (* DeltaSeconds (Variables|Player|GetregenStamina)) (Variables|Player|GetStamineDash)))
    (Variables|Player|SetStamineDash (+ (* DeltaSeconds (Variables|Player|GetregenStamina)) (Variables|Player|GetStamineDash)))))

(fn ConstructionScript)

(fn SetState
  (params (NewState :type EPlayerState%20Enum :default "NewEnumerator0"))
  (bind _output_get (Variables|Player|CachedPlayer|SetStateCurrent NewState))
  (Development|PrintString (Utilities|String|Append "[Player]New State =" (Utilities|String|EnumtoString _output_get))))

(fn GetState
  (return (Variables|Player|CachedPlayer|GetStateCurrent)))

(fn DoJump
  (Character|LaunchCharacter (Math|Vector|MakeVector 0.0 0.0 (Variables|Player|GetJumpForce)) false false)
  (CallFunction|SetState "NewEnumerator2"))

(fn UpdateHorizontalMovement
  (params (MvtForward :type Float%20%28single-precision%29) (MvtRight :type Float%20%28single-precision%29) (sprint :type Boolean))
  (bind _sprintspeed (Variables|Player|GetSPrintSpeed))
  (Utilities|FlowControl|Sequence
    (:then_0
      (Variables|/Script/Engine.CharacterMovementComponent|SetMaxWalkSpeed (Variables|Character|GetCharacterMovement) (select sprint _sprintspeed (Variables|Player|GetMvtSpeedForward)))
      (Pawn|Input|AddMovementInput (Transformation|GetActorForwardVector) (* MvtForward _sprintspeed) false))
    (:then_1
      (Pawn|Input|AddMovementInput (Transformation|GetActorRightVector) (* (Variables|Player|GetMvtSpeedRight) MvtRight) false))))

(fn UpdateAiming
  (params (RotationVertical :type Float%20%28single-precision%29) (RotationHorizontal :type Float%20%28single-precision%29))
  (bind _returnvalue (Pawn|GetController))
  (bind _returnvalue_2 (Pawn|GetControlRotation _returnvalue :!class /Script/Engine.Controller))
  (Utilities|FlowControl|Sequence
    (:then_0
      (LocalVariables|SetL_rotVertical (* (Variables|Aiming|GetAimSpeedVertical) RotationVertical)))
    (:then_1
      (LocalVariables|SetL_rotHorizontal (* (Variables|Aiming|GetAimSpeedHorizontal) RotationHorizontal)))
    (:then_2
      (Pawn|SetControlRotation _returnvalue (Math|Rotator|MakeRotator 0.0 (+ (.pitch _returnvalue_2) (LocalVariables|GetL_rotVertical)) (+ (.yaw _returnvalue_2) (LocalVariables|GetL_rotHorizontal)))))))

(fn DoDash
  (if (<= (Variables|Player|GetcostDash) (Variables|Player|GetStamineDash))
    (Character|LaunchCharacter (* (Math|Vector|GetForwardVector (Variables|Default|GetCamera)) (Variables|Player|GetDashForce)) false false)
    (Variables|Player|SetStamineDash (- (Variables|Player|GetStamineDash) (Variables|Player|GetcostDash)))))

(fn InitPlayer
  (Utilities|FlowControl|Sequence
    (:then_0
      (Default|InitGravityGun (Variables|Default|GetBPC_GravityGun) self))
    (:then_1
      (Variables|Player|CachedPlayer|SetHealthCurrent (Variables|Player|GetHealthMax)))
    (:then_2
      (Variables|Player|CachedPlayer|SetNbKeysCurrent 0))
    (:then_3
      (CallFunction|SetState "NewEnumerator0"))))

(fn GetHealth
  (return (Variables|Player|CachedPlayer|GetHealthCurrent)))

(fn AddHealth
  (params (Health :type Float%20%28single-precision%29))
  (Variables|Player|CachedPlayer|SetHealthCurrent (Math|Float|Clamp(Float) (+ (Variables|Player|CachedPlayer|GetHealthCurrent) Health) 0.0 (Variables|Player|GetHealthMax)))
  (Development|PrintString (Utilities|String|Append "Health=" (Utilities|String|ToString(Float) (Health|GetHealth)))))

(fn TakeDamageInterface
  (params (Damage :type Float%20%28single-precision%29))
  (bind _output_get (Variables|Player|CachedPlayer|SetHealthCurrent (- (Variables|Player|CachedPlayer|GetHealthCurrent) Damage)))
  (if (<= _output_get 0.0)
    (CallFunction|SetState "NewEnumerator3")
    (else
      (Development|PrintString (Utilities|String|Append "Health=" (Utilities|String|ToString(Float) (Health|GetHealth)))))))

(fn Debug
  (Health|TakeDamageInterface 2e+01))

(fn AddKeys
  (params (NbKeys :type Integer))
  (if (> NbKeys 0)
    (Variables|Player|CachedPlayer|SetNbKeysCurrent (+ (Variables|Player|CachedPlayer|GetNbKeysCurrent) NbKeys))
    (else
      (Development|PrintString (Utilities|String|Append "Erreur on ne peut pas ajoute" (Utilities|String|ToString(Integer) NbKeys) "Keys") true true "(R=0.008735,G=1.000000,B=0.000000,A=1.000000)"))))

(fn RemoveKeys
  (params (NbKeys :type Integer))
  (if (> NbKeys 0)
    (if (>= (- (Variables|Player|CachedPlayer|GetNbKeysCurrent) NbKeys) 0)
      (Variables|Player|CachedPlayer|SetNbKeysCurrent (- (Variables|Player|CachedPlayer|GetNbKeysCurrent) NbKeys))
      (else
        (Development|PrintString "trop de key remove" true true "(R=0.008735,G=1.000000,B=0.000000,A=1.000000)")))
    (else
      (Development|PrintString (Utilities|String|Append "Erreur on ne peut pas remove" (Utilities|String|ToString(Integer) NbKeys) "Keys") true true "(R=0.008735,G=1.000000,B=0.000000,A=1.000000)"))))

(fn HasKey
  (return (> (Variables|Player|CachedPlayer|GetNbKeysCurrent) 0)))

(fn GetGrabSocket
  (return (Variables|Default|GetGravityGrabSocket)))

(fn OnGravityGrabPressed
  (Default|OnGrabPressed (Variables|Default|GetBPC_GravityGun)))

(fn OnGravityThrowPressed
  (Default|OnThrowPressed (Variables|Default|GetBPC_GravityGun)))

(fn ForceTransform
  (params (New%20Transform :type Transform))
  (bind (_location _rotation) (Math|Transform|BreakTransform New%20Transform))
  (Utilities|FlowControl|Sequence
    (:then_0
      (Transformation|SetActorLocation (+ _location (* (Variables|/Script/Engine.SceneComponent|GetRelativeLocation (Variables|Default|GetBody)) -1.0)) false true))
    (:then_1
      (Pawn|SetControlRotation (Pawn|GetController) _rotation))))